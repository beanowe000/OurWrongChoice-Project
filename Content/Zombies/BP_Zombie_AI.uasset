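; Zombie enemy that wanders, chases the player on sight, deals contact damage and can be killed.
; A looping AIMoveTo picks random reachable points, while PawnSensing triggers a chase that plays an attack montage on arrival, throttled by its length.
; Damage is separate from the montage: capsule overlap with a "player"-tagged actor runs a repeating timer until overlap ends.
; Incoming damage lowers clamped Health, destroying the zombie at zero.
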(event OnSeePawn(PawnSensing)
  (params (Pawn :type Pawn%20Object%20Reference))
  (Variables|Default|SetIsSeeingPlayer? true)
  (CallFunction|FollowPlayer))

(event OnHearNoise(PawnSensing)
  (params (Instigator :type Pawn%20Object%20Reference) (Location :type Vector%20%28by%20ref%29 :default "0, 0, 0") (Volume :type Float%20%28single-precision%29)))

(event OnComponentBeginOverlap(Capsule)
  (params (OverlappedComponent :type Primitive%20Component%20Object%20Reference) (OtherActor :type Actor%20Object%20Reference) (OtherComp :type Primitive%20Component%20Object%20Reference) (OtherBodyIndex :type Integer) (bFromSweep :type Boolean) (SweepResult :type Hit%20Result%20Structure%20%28by%20ref%29))
  ;[1 0.4271 0.4271] damage player
  (if (Actor|ActorHasTag OtherActor "player")
    (bind _returnvalue (Utilities|Time|SetTimerbyEvent (delegate Custom|Damage) 1.0 true))
    (Variables|Default|SetREF%20Timer _returnvalue)))

(event OnComponentEndOverlap(Capsule)
  (params (OverlappedComponent :type Primitive%20Component%20Object%20Reference) (OtherActor :type Actor%20Object%20Reference) (OtherComp :type Primitive%20Component%20Object%20Reference) (OtherBodyIndex :type Integer))
  ;[1 0.4271 0.4271] damage player
  (if (Actor|ActorHasTag OtherActor "player")
    (Utilities|Time|ClearandInvalidateTimerbyHandle (Variables|Default|GetREF%20Timer))))

(event Custom|FollowPlayer
  ;[0.4787 1 0.9801] Go To Player
  (if (Variables|Default|GetIsSeeingPlayer?)
    (AI|AIMoveTo self "0, 0, 0" (Game|GetPlayerCharacter 0) 7e+01 false
      (:OnSuccess
        (if (Variables|Default|GetCanAttack?)
          (Variables|Default|SetCanAttack? false)
          (bind _returnvalue (Animation|PlayAnimMontage "/Game/Zombies/Zombie_Attack_Montage.Zombie_Attack_Montage" 1.0 "None"))
          (Utilities|FlowControl|Delay _returnvalue)
          (Variables|Default|SetCanAttack? true))))))

(event Custom|Move
  (AI|AIMoveTo self (.RandomLocation (AI|Navigation|GetRandomReachablePointinRadius (Transformation|GetActorLocation) 3e+03 0 0)) 0 5.0 false
    (:OnSuccess
      (Utilities|FlowControl|Delay 5.0)
      ;[1 0.4271 0.4271] damage player
      (CallFunction|Move))))

(event Custom|Damage
  ;[1 0.4271 0.4271] damage player
  (Game|Damage|ApplyDamage (Variables|Default|GetAs%20BP%20Third%20Person%20Character) 5.0 0 self)
  (Audio|PlaySoundatLocation "/Game/ThirdPerson/Blueprints/416839__tonsil5__grunt1-death-pain.416839__tonsil5__grunt1-death-pain" "0, 0, 0" "0, 0, 0" 1.0 1.0 0.0 0 0 0 0))

(event Game|Damage|EventAnyDamage
  (params (Damage :type Float%20%28single-precision%29) (DamageType :type Damage%20Type%20Object%20Reference) (InstigatedBy :type Controller%20Object%20Reference) (DamageCauser :type Actor%20Object%20Reference))
  (bind _returnvalue (Transformation|GetActorLocation))
  (bind _output_get (Variables|Default|SetHealth (Math|Float|Clamp(Float) (- (Variables|Default|GetHealth) Damage) 0.0 1e+02)))
  (if (== _output_get 0.0)
    (Audio|PlaySoundatLocation "/Game/Zombies/396797__scorpion67890__mutant-scream.396797__scorpion67890__mutant-scream" _returnvalue "0, 0, 0" 0.6 1.0 0.0 0 0 0 0)
    (Actor|DestroyActor)
    (else
      (Audio|PlaySoundatLocation 0 _returnvalue "0, 0, 0" 1.0 1.0 0.0 0 0 0 0))))

(event Collision|EventActorBeginOverlap
  (params (OtherActor :type Actor%20Object%20Reference)))

(event EventTick
  (params (DeltaSeconds :type Float%20%28single-precision%29)))

(event EventBeginPlay
  (Utilities|FlowControl|Sequence
    (:then_0
      (bind _asbp_third_person_character (Utilities|Casting|CastToBP_ThirdPersonCharacter (Game|GetPlayerCharacter 0)))
      (Variables|Default|SetAs%20BP%20Third%20Person%20Character _asbp_third_person_character))
    (:then_1
      (CallFunction|Move))))

(fn ConstructionScript)